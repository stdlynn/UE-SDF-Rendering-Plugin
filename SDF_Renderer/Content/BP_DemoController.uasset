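; BP_DemoController is a demo controller that places subtractive or additive SDFs in front of the player's camera.
; Left mouse press spawns an SDF with the subtractive settings, and right mouse press spawns one with the additive settings.
; Both compute the spawn point by projecting PlaceDistance along the camera's forward vector from its location, with no trace.
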(event `Key|LeftMouseButton`
  (params (Key :type "Key Structure"))
  (bind _returnvalue (`GameplayStatics.GetPlayerCameraManager` 0))
  (:`Pressed`
    (`SDFPluginLibrary.SpawnSDF` (+ (`PlayerCameraManager.GetCameraLocation` _returnvalue) (* (`KismetMathLibrary.GetForwardVector` (`PlayerCameraManager.GetCameraRotation` _returnvalue)) (`self.PlaceDistance`))) (`self.SubtractiveSDF`))))

(event `Key|RightMouseButton`
  (params (Key :type "Key Structure"))
  (bind _returnvalue (`GameplayStatics.GetPlayerCameraManager` 0))
  (:`Pressed`
    (`SDFPluginLibrary.SpawnSDF` (+ (`PlayerCameraManager.GetCameraLocation` _returnvalue) (* (`KismetMathLibrary.GetForwardVector` (`PlayerCameraManager.GetCameraRotation` _returnvalue)) (`self.PlaceDistance`))) (`self.AdditiveSDF`))))

(fn `UserConstructionScript`)